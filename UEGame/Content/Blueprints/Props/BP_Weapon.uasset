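; BP_Weapon is a pickup weapon that a BP_Warrior collects on overlap and that damages actors it hits.
; Its Sphere trigger passes the weapon to the warrior's OnWeaponCollected, then disables its own collision.
; AttackCollision starts disabled and is toggled by attack-check begin and end events, applying Damage to any actor it overlaps, with player controller 0 as instigator.
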(event OnComponentBeginOverlap(Sphere)
  (params (OverlappedComponent :type Primitive%20Component%20Object%20Reference) (OtherActor :type Actor%20Object%20Reference) (OtherComp :type Primitive%20Component%20Object%20Reference) (OtherBodyIndex :type Integer) (bFromSweep :type Boolean) (SweepResult :type Hit%20Result%20Structure%20%28by%20ref%29))
  (bind _asbp_warrior (Utilities|Casting|CastToBP_Warrior OtherActor))
  (Default|OnWeaponCollected _asbp_warrior self)
  (Collision|SetCollisionEnabled (Variables|Default|GetSphere) "NoCollision"))

(event OnComponentBeginOverlap(AttackCollision)
  (params (OverlappedComponent :type Primitive%20Component%20Object%20Reference) (OtherActor :type Actor%20Object%20Reference) (OtherComp :type Primitive%20Component%20Object%20Reference) (OtherBodyIndex :type Integer) (bFromSweep :type Boolean) (SweepResult :type Hit%20Result%20Structure%20%28by%20ref%29))
  (Game|Damage|ApplyDamage OtherActor (Variables|Default|GetDamage) (Game|GetPlayerController 0) self))

(event Custom|OnAttackCheckBegin
  (Collision|SetCollisionEnabled (Variables|Default|GetAttackCollision) "QueryOnly"))

(event Custom|OnAttackCheckEnd
  (Collision|SetCollisionEnabled (Variables|Default|GetAttackCollision) "NoCollision"))

(event EventBeginPlay
  (Collision|SetCollisionEnabled (Variables|Default|GetAttackCollision) "NoCollision"))

(event Collision|EventActorBeginOverlap
  (params (OtherActor :type Actor%20Object%20Reference)))

(event EventTick
  (params (DeltaSeconds :type Float%20%28single-precision%29)))

(fn ConstructionScript)