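; BP_MonsterBear is a monster bear that reacts visually when another actor overlaps it.
; BeginPlay creates a dynamic instance of the stone bear material on its mesh.
; An overlap shakes the player camera and plays the HitEffect timeline, which drives the material's HitValue parameter as a hit effect.
; Pawn sensing only prints the seen pawn's name, with no further behavior.
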(event OnSeePawn(PawnSensing)
  (params (Pawn :type Pawn%20Object%20Reference))
  (Development|PrintString (Utilities|GetDisplayName Pawn)))

(event EventBeginPlay
  (bind _returnvalue (Rendering|Material|CreateDynamicMaterialInstance (Variables|Character|GetMesh) 0 "/Game/InfinityBladeAdversaries/Enemy/Enemy_Bear/Materials/M_Bear_Stone_Inst.M_Bear_Stone_Inst" "None" :!class /Script/Engine.PrimitiveComponent))
  (Variables|Default|SetDynamicInstance _returnvalue))

(event Collision|EventActorBeginOverlap
  (params (OtherActor :type Actor%20Object%20Reference))
  (CameraShakes|StartCameraShake (Game|GetPlayerCameraManager 0) "/Game/Blueprints/Warrior/BP_Shake.BP_Shake_C" 1.0 "CameraLocal" "0, 0, 0")
  (bind _effectvalue (Timeline|HitEffect PlayFromStart)
    (:Update
      (Rendering|Material|SetScalarParameterValue (Variables|Default|GetDynamicInstance) "HitValue" _effectvalue :!class /Script/Engine.MaterialInstanceDynamic))))

(fn ConstructionScript)