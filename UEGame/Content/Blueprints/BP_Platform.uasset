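; BP_Platform is a moving platform actor that slides along the direction of its Arrow component.
; On BeginPlay it stores its starting location and plays the Move timeline.
; Each timeline update offsets the actor from that origin by the Alpha track times MoveLength along the arrow's forward vector, without sweeping.
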(event EventBeginPlay
  (Variables|Default|SetOriginLocation (.location (Transformation|GetActorTransform)))
  (bind _alpha (Timeline|Move Play)
    (:Update
      (Transformation|SetActorLocation (+ (Variables|Default|GetOriginLocation) (* (* _alpha (Variables|Default|GetMoveLength)) (Math|Vector|GetForwardVector (Variables|Default|GetArrow)))) false false))))

(fn ConstructionScript)